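; MilhoMan player character for a 2D side-scroller, with horizontal movement, jumping, wall jumps and lives.
; Input flips control yaw to face movement and drives a state-based flipbook switch, with idle standing in for running.
; When a normal jump is unavailable, a box trace detects walls and launches along the hit normal.
; Damage respects an invulnerability window, updates the UI, applies knockback, briefly disables input, and opens "BeginPlay" level at zero lives.
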(event Custom|Update%20Animation
  (switch Utilities|FlowControl|Switch|SwitchonAnimationStates (Variables|Default|GetAnimation%20State)
    (:NewEnumerator1
      (Sprite|SetFlipbook (Variables|Default|GetSprite) (select (> (Math|Vector|VectorLength (Variables|/Script/Engine.MovementComponent|GetVelocity (Variables|Character|GetCharacterMovement))) 0.0) "/Game/Blueprints/1-MilhoMan/Textures/MM-Iddle/A-Iddle.A-Iddle" "/Game/Blueprints/1-MilhoMan/Textures/MM-Iddle/A-Iddle.A-Iddle")))
    (:NewEnumerator2
      (Sprite|SetFlipbook (Variables|Default|GetSprite) "/Game/Blueprints/1-MilhoMan/Textures/A-Jumping.A-Jumping"))
    (:NewEnumerator4
      (Sprite|SetFlipbook (Variables|Default|GetSprite) "/Game/Blueprints/1-MilhoMan/Textures/A-Hit.A-Hit"))))

(event EventOnLanded
  (params (Hit :type Hit%20Result%20Structure%20%28by%20ref%29))
  (Variables|Default|SetAnimation%20State "NewEnumerator1"))

(event Input|ActionEvents|InputActionJump
  (params (Key :type Key%20Structure))
  (:Pressed
    (if (Character|CanJump)
      (Character|Jump)
      (else
        (CallFunction|WallJump)))
    (Variables|Default|SetAnimation%20State "NewEnumerator2"))
  (:Released
    (Character|StopJumping)))

(event Input|AxisEvents|InputAxisHorizontalinput
  (params (AxisValue :type Float%20%28single-precision%29))
  (bind _returnvalue (Pawn|GetController))
  (Pawn|Input|AddMovementInput "1.000000, 0, 0" AxisValue false)
  (CallFunction|UpdateAnimation)
  (Math|Float|CompareFloat AxisValue 0.0
    (:>
      (Pawn|SetControlRotation _returnvalue (Math|Rotator|MakeRotator 0.0 0.0 0.0)))
    (:<
      (Pawn|SetControlRotation _returnvalue (Math|Rotator|MakeRotator 0.0 0.0 1.8e+02)))))

(event Game|Damage|EventAnyDamage
  (params (Damage :type Float%20%28single-precision%29) (DamageType :type Damage%20Type%20Object%20Reference) (InstigatedBy :type Controller%20Object%20Reference) (DamageCauser :type Actor%20Object%20Reference))
  (bind _charactermovement (Variables|Character|GetCharacterMovement))
  ;[1 1 1] Prevent player from taking sucessive damage after being damaged
  (bind _output_get (Variables|LifeManager|SetDamagable (> (Utilities|Time|GetTimeSeconds) (+ (Variables|LifeManager|GetDamageTimer) (Variables|LifeManager|GetIvulnerableTime)))))
  (if _output_get
    (Variables|LifeManager|SetDamageTimer (Utilities|Time|GetTimeSeconds))
    ;[1 1 1] Set new Life ammount and update UI
    (bind _output_get_2 (Variables|LifeManager|SetLives (- (Variables|LifeManager|GetLives) 1.0)))
    (Default|UpdateUI (Variables|LifeManager|GetUI) _output_get_2)
    ;[1 1 1] update animation
    (Variables|Default|SetAnimation%20State "NewEnumerator4")
    (CallFunction|UpdateAnimation)
    ;[1 1 1] //BUG - if mik damage you and he is fast enought to maintain you inside his dagame trigger you can reach the enable input again//handles movemente after taking damage
    (Math|Float|CompareFloat (.x (Variables|/Script/Engine.MovementComponent|GetVelocity (Variables|Character|GetCharacterMovement))) 0.0
      (:>
        (Physics|AddImpulse _charactermovement "-350.000000,0.0,200.0" true :!label _label))
      (:==
        (goto _label))
      (:<
        (Physics|AddImpulse _charactermovement "350.000000,0.0,200.0" true)))
    (Input|DisableInput 0)
    (Utilities|FlowControl|Delay 0.2)
    (Input|EnableInput 0)
    ;[1 1 1] Update animation
    (Variables|Default|SetAnimation%20State "NewEnumerator1")
    (CallFunction|UpdateAnimation)
    ;[1 1 1] //TODO On death to someting
    (if (< (Variables|LifeManager|GetLives) 0.1)
      (Utilities|FlowControl|Delay 0.2)
      (Game|OpenLevel(byName) "BeginPlay"))))

(event EventBeginPlay
  ;[1 1 1] Setup Initial Lives
  (Variables|LifeManager|SetLives (Variables|LifeManager|GetInitialLives))
  ;[1 1 1] setup DamageTimer
  (Variables|LifeManager|SetDamageTimer (- (Utilities|Time|GetTimeSeconds) (Variables|LifeManager|GetIvulnerableTime)))
  (bind _returnvalue (UserInterface|CreateWidget "/Game/Widgets/UI.UI_C"))
  (bind _output_get (Variables|LifeManager|SetUI _returnvalue))
  (UserInterface|Viewport|AddtoViewport _output_get 0))

(fn ConstructionScript)

(fn WallJump
  ;[1 1 1] // TODO restric player input just after a succesful wall jump (so the player has time to change the direction pressed on horizontal axis without impair the wall jump magic)
  (bind (_wallsliding _wallnormal) (CallFunction|IsWallSliding?))
  (if _wallsliding
    (Physics|AddImpulse (Variables|Character|GetCharacterMovement) (Math|Vector|MakeVector (* _wallnormal 2.5e+02) 0.0 4.5e+02) true)))

(fn IsWallSliding?
  (bind _returnvalue (Transformation|GetActorLocation))
  ;[1 1 1] //TODO refine volume as player model evolves
  (bind (_outhit _returnvalue_2) (Collision|BoxTraceByChannel _returnvalue (+ _returnvalue "0, 0,-1.000000") "22.000000,0.000000,20.000000" "0, 0, 0" "TraceTypeQuery1" false 0 "ForDuration"))
  (return _returnvalue_2 (.X (Math|Vector|BreakVector (.Normal (Collision|BreakHitResult _outhit))))))