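; MilhoMan player actor: a physics-driven Paper2D side-scroller character with running, jumping, wall jumping and lives.
; Forces drive horizontal movement and braking; impulses drive jumps, cut short on early release.
; Three line traces detect ground, a box trace supplies the wall-jump normal, and OverrideJump briefly permits an extra jump.
; Damage respects an invulnerability window, updates the UI, stops and blinks the character, then opens level "BeginPlay" when lives run out.
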(event EventTick
  (params (DeltaSeconds :type Float%20%28single-precision%29))
  ;[1 1 1] //TODO Jump on miks head //TODO Please refactor this and on Rep kill Jump and Mik firning all this shit
  (if (Variables|Default|GetOverride%20jump)
    (Utilities|FlowControl|Delay 0.1)
    (Variables|Default|SetOverride%20jump false)))

(event Input|ActionEvents|InputActionJump
  (params (Key :type Key%20Structure))
  ;[1 1 1] //TODO Jump on miks head //TODO Please refactor this and on Rep kill Jump and Mik firning all this shit
  (:Pressed
    (if (Variables|Default|GetOverride%20jump)
      (Physics|AddImpulse (Variables|Default|GetPaperSprite) (Math|Vector|MakeVector 0.0 0.0 (* 0.7 (Variables|InputController|GetJumpInitialForce))) "None" true))))

(event Input|ActionEvents|InputActionJump
  (params (Key :type Key%20Structure))
  (:Pressed
    ;[1 1 1] Jump if is grounded and not falling, but if both is true than add ashort delay to make the jump (//TODO maybe loop for finite time to chek if is falling yet - this will improve precision)
    (bind _isgrounded (CallFunction|IsGrounded))
    (if _isgrounded
      (bind _isfalling_ (CallFunction|IsFalling))
      (if _isfalling_
        (Utilities|FlowControl|Delay 0.015))
      (Physics|AddImpulse (Variables|Default|GetPaperSprite) (Math|Vector|MakeVector 0.0 0.0 (Variables|InputController|GetJumpInitialForce)) "None" true)
      (else
        (CallFunction|WallJump))))
  (:Released
    ;[1 1 1] ADD force restricting jump max height if jump button is released early
    (bind _returnvalue (Physics|GetPhysicsLinearVelocity (Variables|Default|GetPaperSprite) "None"))
    (if (> (.Z (Math|Vector|BreakVector _returnvalue)) 0.0)
      (Physics|AddImpulse (Variables|Default|GetPaperSprite) (Math|Vector|MakeVector 0.0 0.0 (* (.Z (Math|Vector|BreakVector _returnvalue)) -2.0)) "None" false))))

(event Input|AxisEvents|InputAxisHorizontalinput
  (params (AxisValue :type Float%20%28single-precision%29))
  ;[1 1 1] Move Horizontal
  (CallFunction|MoveHorizontal AxisValue))

(event Game|Damage|EventAnyDamage
  (params (Damage :type Float%20%28single-precision%29) (DamageType :type Damage%20Type%20Object%20Reference) (InstigatedBy :type Controller%20Object%20Reference) (DamageCauser :type Actor%20Object%20Reference))
  ;[1 1 1] Prevent player from taking sucessive damage after being damaged
  (bind _output_get (Variables|LifeManager|SetDamagable (> (Utilities|Time|GetTimeSeconds) (+ (Variables|LifeManager|GetDamageTimer) (Variables|LifeManager|GetIvulnerableTime)))))
  (if _output_get
    (Variables|LifeManager|SetDamageTimer (Utilities|Time|GetTimeSeconds))
    ;[1 1 1] Set new Life ammount and update UI
    (bind _output_get_2 (Variables|LifeManager|SetLives (- (Variables|LifeManager|GetLives) 1.0)))
    (Default|UpdateUI (Variables|LifeManager|GetUI) _output_get_2)
    (Physics|SetPhysicsLinearVelocity (Variables|Default|GetPaperSprite) "0, 0, 0" false "None")
    (Rendering|ToggleVisibility (Variables|Default|GetPaperFlipbook) false)
    (Utilities|FlowControl|Delay 0.1)
    (Physics|SetPhysicsLinearVelocity (Variables|Default|GetPaperSprite) "0, 0, 0" false "None")
    (Rendering|ToggleVisibility (Variables|Default|GetPaperFlipbook) false)
    (Utilities|FlowControl|Delay 0.1)
    ;[1 1 1] //TODO On death to someting
    (if (< (Variables|LifeManager|GetLives) 0.1)
      (Game|OpenLevel(byName) "BeginPlay"))))

(event EventBeginPlay
  ;[1 1 1] Setup Initial Lives
  (Variables|LifeManager|SetLives (Variables|LifeManager|GetInitialLives))
  ;[1 1 1] setup DamageTimer
  (Variables|LifeManager|SetDamageTimer (- (Utilities|Time|GetTimeSeconds) (Variables|LifeManager|GetIvulnerableTime)))
  (bind _returnvalue (UserInterface|CreateWidget "/Game/Widgets/UI.UI_C"))
  (bind _output_get (Variables|LifeManager|SetUI _returnvalue))
  (UserInterface|Viewport|AddtoViewport _output_get 0))

(fn ConstructionScript)

(fn MoveHorizontal
  (params (Axis%20Value :type Float%20%28single-precision%29))
  (bind _output_get (Variables|InputController|SetHorizontal%20Axis Axis%20Value))
  (if (!= _output_get 0.0)
    ;[1 1 1] Check if velocity is < than max velocity // check if input is reverting movement
    (bind _returnvalue (Physics|GetPhysicsLinearVelocity (Variables|Default|GetPaperSprite) "None"))
    (if (or (> (Variables|InputController|GetMaxFowardVelocity) (Math|Float|Absolute(Float) (.X (Math|Vector|BreakVector _returnvalue)))) (< (* (.X (Math|Vector|BreakVector _returnvalue)) (Variables|InputController|GetHorizontal%20Axis)) 0.0))
      ;[1 1 1] Apply force to walk
      (Physics|AddForce (Variables|Default|GetPaperSprite) (Math|Vector|MakeVector (* (Variables|InputController|GetHorizontal%20Axis) (Variables|InputController|GetMaxFowardVelocity) (Variables|InputController|GetMaxVel%20Force%20Rate)) 0.0 0.0) "None" true))
    (else
      ;[1 1 1] if no input, than add restitution force to make player stop moving in X axis
      (bind _returnvalue_2 (Physics|GetPhysicsLinearVelocity (Variables|Default|GetPaperSprite) "None"))
      (if (!= (.X (Math|Vector|BreakVector _returnvalue_2)) 0.0)
        (Physics|AddForce (Variables|Default|GetPaperSprite) (Math|Vector|MakeVector (* (.X (Math|Vector|BreakVector _returnvalue_2)) (Variables|InputController|GetFrictionFactor)) 0.0 0.0) "None" true)))))

(fn IsGrounded
  (bind _returnvalue (Transformation|GetActorLocation))
  ;[1 1 1] //TODO refactor this shit - its awful but works for now
  (bind _returnvalue_2 (Collision|LineTraceByChannel _returnvalue (+ _returnvalue "0.000000, 0,-36.500000") "TraceTypeQuery1" false 0 "ForDuration"))
  (bind _returnvalue_3 (Collision|LineTraceByChannel (+ _returnvalue "14.000000,0.000000,0.000000") (+ _returnvalue "14.000000,0.000000,-36.500000") "TraceTypeQuery1" false 0 "ForDuration"))
  (bind _returnvalue_4 (Collision|LineTraceByChannel (+ _returnvalue "-10.000000, 0,0.000000") (+ _returnvalue "-10.000000, 0,-36.500000") "TraceTypeQuery1" false 0 "ForDuration"))
  (return (Math|Boolean|ORBoolean _returnvalue_2 _returnvalue_3 _returnvalue_4)))

(fn IsFalling
  (bind _returnvalue (Physics|GetPhysicsLinearVelocity (Variables|Default|GetPaperSprite) "None"))
  (return (< (.Z (Math|Vector|BreakVector _returnvalue)) -5e+01)))

(fn WallJump
  ;[1 1 1] // TODO restric player input just after a succesful wall jump (so the player has time to change the direction pressed on horizontal axis without impair the wall jump magic)
  (bind (_wallsliding _wallnormal) (CallFunction|IsWallSliding?))
  (if _wallsliding
    (Physics|AddImpulse (Variables|Default|GetPaperSprite) (Math|Vector|MakeVector (* _wallnormal 3.5e+02) 0.0 (Variables|InputController|GetJumpInitialForce)) "None" true)))

(fn IsWallSliding?
  (bind _returnvalue (Transformation|GetActorLocation))
  ;[1 1 1] //TODO refine volume as player model evolves
  (bind (_outhit _returnvalue_2) (Collision|BoxTraceByChannel _returnvalue (+ _returnvalue "0, 0,-1.000000") "22.000000,0.000000,20.000000" "0, 0, 0" "TraceTypeQuery1" false 0 "ForDuration"))
  (return _returnvalue_2 (.X (Math|Vector|BreakVector (.Normal (Collision|BreakHitResult _outhit))))))

(fn OnRepKillJump
  (bind _returnvalue (Transformation|GetVelocity))
  (bind (_x _y) (Math|Vector|BreakVector _returnvalue))
  (Physics|SetPhysicsLinearVelocity (Variables|Default|GetPaperSprite) (Math|Vector|MakeVector _x _y 0.0) false "None")
  (Physics|AddImpulse (Variables|Default|GetPaperSprite) (Math|Vector|MakeVector 0.0 0.0 (/ (Variables|InputController|GetJumpInitialForce) 2.0)) "None" true))