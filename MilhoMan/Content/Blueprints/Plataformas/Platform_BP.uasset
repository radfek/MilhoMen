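; Platform actor that either moves vertically or fades in and out, chosen by its PlatBehaviour setting.
; On BeginPlay, Up/Down plays a timeline that offsets the actor's Z from its starting location, scaled by Distance.
; Fade plays a second timeline that hides the cube and disables actor collision whenever its value equals 1, an on/off switch rather than a gradual opacity change.
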(event EventBeginPlay
  (switch Utilities|FlowControl|Switch|SwitchonPlatformEnum (Variables|PlatformSetup|GetPlat%20Behaviour)
    (:NewEnumerator0
      (Variables|PlatformSetup|SetInitial%20location (Transformation|GetActorLocation))
      (bind _z_position (Timeline|Timeline_0 Play)
        (:Update
          (Transformation|SetActorLocation (+ (Variables|PlatformSetup|GetInitial%20location) (Math|Vector|MakeVector 0.0 0.0 (* _z_position (Variables|PlatformSetup|GetDistance)))) false false))))
    (:NewEnumerator1
      (bind _z_position_2 (Timeline|Timeline_1 Play)
        (:Update
          (Rendering|SetVisibility (Variables|Default|GetCube) (!= _z_position_2 1.0) false)
          (Collision|SetActorEnableCollision (!= _z_position_2 1.0)))))))

(fn ConstructionScript)