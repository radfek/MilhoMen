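; Configurable 2D platform that moves or blinks, with optional one-way pass-through and drop-down.
; On BeginPlay, PlatBehaviour selects a timeline that offsets the actor by Distance vertically or horizontally, or toggles sprite visibility and collision, with reverse variants.
; When CanGoTrhough is set, a trigger box switches the sprite's GameTraceChannel1 response to Block while MM-V3 overlaps.
; It also binds DropPlat on MMController to restore Overlap, letting the player drop through.
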(event OnComponentBeginOverlap(gotroughttriggerbox)
  (params (OverlappedComponent :type Primitive%20Component%20Object%20Reference) (OtherActor :type Actor%20Object%20Reference) (OtherComp :type Primitive%20Component%20Object%20Reference) (OtherBodyIndex :type Integer) (bFromSweep :type Boolean) (SweepResult :type Hit%20Result%20Structure%20%28by%20ref%29))
  (if (Variables|Default|GetCan%20go%20trhough)
    (bind _asmm_v3 (Utilities|Casting|CastToMM-V3 OtherActor))
    (Collision|SetCollisionResponsetoChannel (Variables|Default|GetPaperSprite) "ECC_GameTraceChannel1" "ECR_Block")
    ;[1 1 1] drop plat
    (bind _asmmcontroller (Utilities|Casting|CastToMMController (Pawn|GetController _asmm_v3)))
    (EventDispatchers|BindEventtoDropPlat _asmmcontroller (delegate Custom|Drop%20plat))))

(event OnComponentEndOverlap(gotroughttriggerbox)
  (params (OverlappedComponent :type Primitive%20Component%20Object%20Reference) (OtherActor :type Actor%20Object%20Reference) (OtherComp :type Primitive%20Component%20Object%20Reference) (OtherBodyIndex :type Integer))
  (if (Variables|Default|GetCan%20go%20trhough)
    (Utilities|Casting|CastToMM-V3 OtherActor)
    (Collision|SetCollisionResponsetoChannel (Variables|Default|GetPaperSprite) "ECC_GameTraceChannel1" "ECR_Overlap")))

(event Custom|Drop%20plat
  ;[1 1 1] drop plat
  (Collision|SetCollisionResponsetoChannel (Variables|Default|GetPaperSprite) "ECC_GameTraceChannel1" "ECR_Overlap"))

(event EventBeginPlay
  (bind _papersprite (Variables|Default|GetPaperSprite))
  (if (Variables|Default|GetCan%20go%20trhough)
    (Collision|SetCollisionResponsetoChannel _papersprite "ECC_GameTraceChannel1" "ECR_Overlap")
    (else
      (Collision|SetCollisionResponsetoChannel _papersprite "ECC_GameTraceChannel1" "ECR_Block")))
  (switch Utilities|FlowControl|Switch|SwitchonPlatform-MovingModes (Variables|PlatformSetup|GetPlat%20Behaviour)
    (:NewEnumerator0
      ;[1 1 1] Vertical movement
      (Variables|PlatformSetup|SetInitial%20location (Transformation|GetActorLocation))
      (bind _z_position (Timeline|Timeline_0 Play)
        (:Update
          (Transformation|SetActorLocation (+ (Variables|PlatformSetup|GetInitial%20location) (Math|Vector|MakeVector 0.0 0.0 (* _z_position (Variables|PlatformSetup|GetDistance)))) false false))))
    (:NewEnumerator5
      (Variables|PlatformSetup|SetInitial%20location (Transformation|GetActorLocation))
      (bind _z_position_2 (Timeline|Timeline_3 Play)
        (:Update
          (Transformation|SetActorLocation (- (Variables|PlatformSetup|GetInitial%20location) (Math|Vector|MakeVector 0.0 0.0 (* _z_position_2 (Variables|PlatformSetup|GetDistance)))) false false))))
    (:NewEnumerator2
      ;[1 1 1] Horizontal movement
      (Variables|PlatformSetup|SetInitial%20location (Transformation|GetActorLocation))
      (bind _x_position (Timeline|Timeline_2 Play)
        (:Update
          (Transformation|SetActorLocation (+ (Variables|PlatformSetup|GetInitial%20location) (Math|Vector|MakeVector (* _x_position (Variables|PlatformSetup|GetDistance)) 0.0 0.0)) false false))))
    (:NewEnumerator6
      ;[1 1 1] Horizontal movement
      (Variables|PlatformSetup|SetInitial%20location (Transformation|GetActorLocation))
      (bind _x_position_2 (Timeline|Timeline_4 Play)
        (:Update
          (Transformation|SetActorLocation (- (Variables|PlatformSetup|GetInitial%20location) (Math|Vector|MakeVector (* _x_position_2 (Variables|PlatformSetup|GetDistance)) 0.0 0.0)) false false))))
    (:NewEnumerator1
      ;[1 1 1] Fading platform // TODO add a exposed variable to set diferent initial times
      (bind _z_position_3 (Timeline|Timeline_1 Play)
        (:Update
          (Rendering|SetVisibility (Variables|Default|GetPaperSprite) (!= _z_position_3 1.0) true)
          (Collision|SetActorEnableCollision (!= _z_position_3 1.0)))))
    (:NewEnumerator4
      (Timeline|Timeline_1 Reverse))))

(fn ConstructionScript)